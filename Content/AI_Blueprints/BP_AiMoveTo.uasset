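; AI enemy Blueprint that repeatedly moves toward the first player controller and varies its skeletal mesh appearance.
; BeginPlay starts an AI MoveTo that targets the controller actor itself, retrying after a short delay on success or failure.
; The first Tick applies a random material through a DoOnce.
; ChangeRandomEnemy and MakeRandomMeshes pick random skeletal meshes from MaterialMeshes, but nothing in this Blueprint calls them.
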(event `self.ReceiveBeginPlay`
  (`|AIMoveTo` self (0.0 0.0 0.0) (`GameplayStatics.GetPlayerController` 0) 200.0 :!label _label
    (:`OnSuccess`
      _)
    (:`OnFail`
      _))
  (`KismetSystemLibrary.Delay` 1.0)
  (goto _label))

(event `ChangeRandomColor`
  (`PrimitiveComponent.SetMaterial` (`self.Mesh`) 0 (`KismetArrayLibrary.Array_Random` (`self.Materials`))))

(event `self.ReceiveTick`
  (params (DeltaSeconds :type "Float (single-precision)"))
  (`|ExecutionSequence`
    (:`then_0`
      (`/Engine/EditorBlueprintResources/StandardMacros.DoOnce` false
        (:`Completed`
          (`self.ChangeRandomColor`))))))

(event `ChangeRandomEnemy`
  (`SkeletalMeshComponent.SetSkeletalMeshAsset` (`self.Mesh`) (`KismetArrayLibrary.Array_Random` (`self.MaterialMeshes`))))

(fn `MakeRandomMeshes`
  (params (NewMesh :type "SkeletalMesh Object Reference"))
  (bind _materialmeshes (`self.MaterialMeshes`))
  (`SkeletalMeshComponent.SetSkeletalMeshAsset` (`self.Mesh`) (`|GetArrayItem` _materialmeshes (`KismetMathLibrary.RandomInteger` (`KismetArrayLibrary.Array_Length` _materialmeshes))))
  (return))

(fn `UserConstructionScript`)