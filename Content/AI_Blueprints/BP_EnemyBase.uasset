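; BP_EnemyBase is a base enemy character exposing attack, aggro, speed, patrol and combat-distance functions, with speed set by behavior tree task BTT_SetSpeed.
; Attacks play a kick montage and signal completion or interruption, while aggro swaps the mesh material to red.
; Point damage drains Health, triggering physics ragdoll with radial force at zero.
; Patrol steps along spline points, but its intended direction flip multiplies by zero, halting advancement.
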(event `self.ReceiveBeginPlay`
  (set `self.Original Material` (`PrimitiveComponent.GetMaterial` (`self.Mesh`) 0)))

(event `Attack`
  (`KismetSystemLibrary.PrintString` "Attacking Player!")
  (`|PlayMontage` (`self.Mesh`) "/Game/CloseCombatAnimSet/Animations/InPlace/Attacks/NinjaWheelKick_Montage.NinjaWheelKick_Montage"
    (:`OnCompleted`
      _)
    (:`OnInterrupted`
      _))
  (`self.AttackedFinished`))

(event `GetAggro`
  (`PrimitiveComponent.SetMaterial` (`self.Mesh`) 0 "/Game/Materials/M_Red.M_Red")
  (set `self.Aggroed` true) ; sets to true
)

(event `LoseAggro`
  (`PrimitiveComponent.SetMaterial` (`self.Mesh`) 0 (`self.Original Material`))
  (set `self.Aggroed` false) ; sets to true
)

(event `Investigating`
  (`KismetSystemLibrary.PrintString` "Investigating "))

(event `setWalkSpeed`
  (params (`New Speed` :type "Float (double-precision)"))
  (set `CharacterMovementComponent.MaxWalkSpeed` `New Speed` (`self.CharacterMovement`)))

(event `self.ReceiveAnyDamage`
  (params (Damage :type "Float (single-precision)") (DamageType :type "DamageType Object Reference") (InstigatedBy :type "Controller Object Reference") (DamageCauser :type "Actor Object Reference")))

(event `self.ReceivePointDamage`
  (params (Damage :type "Float (single-precision)") (DamageType :type "DamageType Object Reference") (HitLocation :type "Vector Structure") (HitNormal :type "Vector Structure") (HitComponent :type "PrimitiveComponent Object Reference") (BoneName :type Name) (ShotFromDirection :type "Vector Structure") (InstigatedBy :type "Controller Object Reference") (DamageCauser :type "Actor Object Reference") (HitInfo :type "HitResult Structure (by ref)"))
  (`KismetSystemLibrary.PrintText` (`|FormatText` "{instigate} damaged for {dmg} damage!" InstigatedBy Damage) true true (struct :`R` 0.748989 :`G` 0.108805 :`B` 1.0 :`A` 1.0) 5.0)
  (bind _output_get (set `self.Health` (- (`self.Health`) Damage)))
  (if (<= _output_get 0.0)
    (`self.Ragdoll` (0.0 0.0 0.0))))

(event `Ragdoll`
  (params (Origin :type "Vector Structure"))
  (bind _mesh (`self.Mesh`))
  (`PrimitiveComponent.SetSimulatePhysics` _mesh true) ; don't forget to change the mesh's collision\npreset to "ragdoll"
  (`PrimitiveComponent.AddRadialForce` _mesh (+ Origin (0.0 0.0 -100.0)) 500.0 50000.0 "RIF_Constant" true) ; strength is not... consistent.
  (`CharacterMovementComponent.DisableMovement` (`self.CharacterMovement`)))

(fn `GetIdealDistance`
  (returns (AttackRadius :type "Float (double-precision)") (StrafeRadius :type "Float (double-precision)"))
  (return (`self.Attack Radius`) (`self.Strafe Radius`)))

(fn `GetNextPatrolPointLocation`
  (returns (Location :type "Vector Structure"))
  (`/Engine/EditorBlueprintResources/StandardMacros.IsValid` (`self.PatrolRoute`)
    (:`Is Valid`
      (set `self.Patrol Point Index` (+ (`self.Patrol Point Index`) (`self.PatrolRouteDirection`))) ; Update next point
      (if (or (>= (`self.Patrol Point Index`) (`SplineComponent.GetNumberOfSplinePoints` (`/Game/Blueprints/BP_PatrolRoute.Spline` (`self.PatrolRoute`)))) (<= (`self.Patrol Point Index`) 1))
        (set `self.PatrolRouteDirection` (* (`self.PatrolRouteDirection`) 0)) ; Flip the direction
      )
      (return (`SplineComponent.GetLocationAtSplinePoint` (`/Game/Blueprints/BP_PatrolRoute.Spline` (`self.PatrolRoute`)) (`self.Patrol Point Index`) "World")))
    (:`Is Not Valid`
      (`KismetSystemLibrary.PrintString` "No Path is assigned"))))

(fn `MakeRandomMeshes`
  (params (NewMesh :type "SkeletalMesh Object Reference"))
  (bind _materialmeshes (`self.MaterialMeshes`))
  (`SkeletalMeshComponent.SetSkeletalMeshAsset` (`self.Mesh`) (`|GetArrayItem` _materialmeshes (`KismetMathLibrary.RandomInteger` (`KismetArrayLibrary.Array_Length` _materialmeshes))))
  (return))

(fn `UserConstructionScript`)