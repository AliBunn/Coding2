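; BP_EnemySpawner populates the level with named AI enemies when play begins.
; It shuffles a name list, then gives each BP_EnemySpawnPoint a weighted coin flip to spawn a BP_AiMoveTo at its transform.
; Each enemy's text render shows the name at that point's index.
; SetMaterial has no material supplied, and the red dynamic material node never runs.
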(event `self.ReceiveBeginPlay`
  (`KismetSystemLibrary.PrintString` "enemy spawner is active")
  (bind _outactors (`GameplayStatics.GetAllActorsOfClass` "/Game/Blueprints/BP_EnemySpawnPoint.BP_EnemySpawnPoint_C"))
  (`KismetArrayLibrary.Array_Shuffle` (`self.names`))
  (for (_array_element _array_index) _outactors
    (if (`KismetMathLibrary.RandomBoolWithWeight` 0.5)
      (bind _returnvalue (`|SpawnActorFromClass` "/Game/AI_Blueprints/BP_AiMoveTo.BP_AiMoveTo_C" (`self.GetTransform` _array_element) "Undefined" "MultiplyWithRoot" null null)) ; spawn actor BP move to (spawn actor from class)
      (`PrimitiveComponent.SetMaterial` (`Character.Mesh` _returnvalue) 0 null)
      (`TextRenderComponent.K2_SetText` (`/Game/AI_Blueprints/BP_AiMoveTo.TextRender` _returnvalue) (`|GetArrayItem` (`self.names`) _array_index))
      (`KismetSystemLibrary.PrintString` "Enemy spawned"))))

(fn `UserConstructionScript`)