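; GM_SavLoad is a game mode that handles saving and loading player stats in the PlayerSave slot.
; On BeginPlay it loads the SG_PlayerStats save and copies its Stamina to the third-person character, or creates a new save object if none exists.
; SavePlayerStats writes the held save object without updating it from the character, and its success message prints regardless of the save result.
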(event `self.ReceiveBeginPlay`
  (`KismetSystemLibrary.PrintString` "Loading the SavLoad Game Mode" true true (struct :`R` 0.169452 :`G` 0.116751 :`B` 1.0 :`A` 1.0))
  (`self.Load Player Stats`))

(event `Load Player Stats`
  (bind _returnvalue (`GameplayStatics.DoesSaveGameExist` "PlayerSave")) ; Slot Name is the save slot of the game
  (if _returnvalue
    (bind _returnvalue_2 (`GameplayStatics.LoadGameFromSlot` "PlayerSave"))
    (bind _assg_player_stats (cast `/Game/Blueprints/SAvingLoading/SG_PlayerStats` _returnvalue_2))
    (set `self.SG_PlayerStats` _assg_player_stats)
    (bind _asbp_third_person_character (cast `/Game/ThirdPerson/Blueprints/BP_ThirdPersonCharacter` (`GameplayStatics.GetPlayerCharacter` 0)))
    (set `/Game/ThirdPerson/Blueprints/BP_ThirdPersonCharacter.Stamina` (`/Game/Blueprints/SAvingLoading/SG_PlayerStats.Stamina` (`self.SG_PlayerStats`)) _asbp_third_person_character) ; The Player's Stamina
    (`KismetSystemLibrary.PrintString` "Hello")
    (else
      (bind _returnvalue_3 (`GameplayStatics.CreateSaveGameObject` "/Game/Blueprints/SAvingLoading/SG_PlayerStats.SG_PlayerStats_C"))
      (set `self.SG_PlayerStats` _returnvalue_3) ; set this variable so thay the \nplayer can edit these values
    )))

(event `Save Player Stats`
  (`GameplayStatics.SaveGameToSlot` (`self.SG_PlayerStats`) "PlayerSave")
  (if true
    (`KismetSystemLibrary.PrintText` "Player Stats Written to Save Game File" true true (struct :`R` 0.125932 :`G` 1.0 :`B` 0.205382 :`A` 1.0))
    (else
      (`KismetSystemLibrary.PrintText` "Player Stats Could Not be Written to Save Game File" true true (struct :`R` 1.0 :`G` 0.043653 :`B` 0.119488 :`A` 1.0)))))

(fn `UserConstructionScript`)