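; Machine gun pickup actor that can be picked up, fired and dropped, with firing only a printed placeholder.
; PickUp prints a debug message, snaps the gun to the hand_r socket of the supplied skeletal mesh and disables body collision.
; Drop detaches it in world space and turns physics simulation off.
; The nodes that re-enable collision and delay a physics shutoff are disconnected, so collision stays off after a drop.
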(event `/Game/Blueprints/BPI_Item.PickUp`
  (params (SkeletalMesh :type "SkeletalMeshComponent Object Reference"))
  ; Pickup Function
  (`KismetSystemLibrary.PrintText` (`|FormatText` "{name} is getting picked up and attached to {mesh}" "Machine Gun" SkeletalMesh))
  (`self.K2_AttachToComponent` SkeletalMesh "hand_r" "SnapToTarget" "SnapToTarget" "SnapToTarget")
  (`PrimitiveComponent.SetCollisionEnabled` (`self.MachineGunBody`) "NoCollision"))

(event `/Game/Blueprints/BPI_Item.UsePrimary`
  (`KismetSystemLibrary.PrintText` "pew pew pew"))

(event `/Game/Blueprints/BPI_Item.Drop`
  (`self.K2_DetachFromActor` "KeepWorld" "KeepWorld" "KeepWorld")
  (`PrimitiveComponent.SetSimulatePhysics` (`self.MachineGunBody`) false))

(fn `UserConstructionScript`)