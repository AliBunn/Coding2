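; Demo Blueprint of loops and arrays that prints colored debug messages to the screen from BeginPlay.
; DelayLoop logs a running counter, waits one second, calls PrintColors, then calls itself again, forming an endless timed loop.
; PrintColors shuffles Textcolors and loops over it, but each line's color is picked randomly from an inline four-color array.
; A few disconnected loop and random-index nodes are left unused.
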(event `self.ReceiveBeginPlay`
  (`KismetSystemLibrary.PrintString` "Loops and List is active.")
  (`self.Delay Loop`) ; Start the delay loop
)

(event `Delay Loop`
  (`KismetSystemLibrary.PrintString` (`KismetStringLibrary.Concat_StrStr` "Starting Delay Loop #" (`KismetStringLibrary.Conv_IntToString` (`self.DelayLoopCounter`))))
  (`/Engine/EditorBlueprintResources/StandardMacros.IncrementInt` (`self.DelayLoopCounter`)
    (:`  `
      (`KismetSystemLibrary.Delay` 1.0)
      (`self.Print Colors`)
      (`self.Delay Loop`))))

(event `Print Colors`
  (bind _textcolors (`self.textcolors`))
  (`KismetArrayLibrary.Array_Shuffle` _textcolors)
  (for (_ _array_index) _textcolors
    (`KismetSystemLibrary.PrintString` (`KismetStringLibrary.Concat_StrStr` "Printing color #" (`KismetStringLibrary.Conv_IntToString` _array_index)) true true (`KismetArrayLibrary.Array_Random` (`|MakeArray` (struct :`R` 1.0 :`G` 0.940761 :`A` 1.0) (struct :`R` 1.0 :`B` 0.017108 :`A` 1.0) (struct :`R` 0.048602 :`G` 1.0 :`A` 1.0) (struct :`G` 0.04929 :`B` 1.0 :`A` 1.0) :!type "LinearColor Structure"))))
  (`KismetSystemLibrary.PrintString` "We are Done Printing Colors!!"))

(fn `UserConstructionScript`)